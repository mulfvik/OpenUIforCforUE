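; Player controller Blueprint that starts in game-only input with the cursor hidden and toggles a main menu widget.
; Space or the gamepad Special Right button flips a boolean, either creating WBP_Main with Game and UI input and a visible cursor, or removing all widgets and hiding the cursor.
; Closing does not restore game-only input, and the ToggleMenu function is empty.
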(event EventBeginPlay
  (Input|SetInputModeGameOnly self true)
  (Variables|Default|SetbShowMouseCursor false))

(event Input|GamepadEvents|GamepadSpecialRight
  (params (Key :type Key%20Structure :default "None"))
  (:Pressed
    (bind _output_get (Variables|Default|SetbMainWidget (not (Variables|Default|GetbMainWidget))))
    (if _output_get
      (bind _returnvalue (UserInterface|CreateWidget "/OpenUIforCforUE/Widgets/WBP_Main.WBP_Main_C"))
      (UserInterface|Viewport|AddtoViewport _returnvalue 0)
      (Input|SetInputModeGameandUI self _returnvalue "DoNotLock" true false)
      (Variables|Default|SetbShowMouseCursor true)
      (else
        (Viewport|RemoveAllWidgets)
        (Variables|Default|SetbShowMouseCursor false)))))

(event Input|KeyboardEvents|SpaceBar
  (params (Key :type Key%20Structure :default "None"))
  (:Pressed
    (bind _output_get (Variables|Default|SetbMainWidget (not (Variables|Default|GetbMainWidget))))
    (if _output_get
      (bind _returnvalue (UserInterface|CreateWidget "/OpenUIforCforUE/Widgets/WBP_Main.WBP_Main_C"))
      (UserInterface|Viewport|AddtoViewport _returnvalue 0)
      (Input|SetInputModeGameandUI self _returnvalue "DoNotLock" true false)
      (Variables|Default|SetbShowMouseCursor true)
      (else
        (Viewport|RemoveAllWidgets)
        (Variables|Default|SetbShowMouseCursor false)))))

(fn ConstructionScript)

(fn ToggleMenu)